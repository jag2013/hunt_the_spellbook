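; A physics-driven spellbook prop that can be picked up, dropped and returned, apparently for a VR game.
; Pickup and drop toggle mesh simulation while attaching or detaching the book.
; Impacts with anything but the player pawn play a slam sound, throttled by a flag and delay.
; Returning it runs once: after a delay it vanishes with a pop and smoke, then destroys the mesh and calls the game mode's respawn message.
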(event Custom|BookReturned
  (bind _spellbook_mesh (Variables|Default|Getspellbook_mesh))
  (bind _returnvalue (Transformation|GetWorldLocation _spellbook_mesh))
  (Utilities|FlowControl|DoOnce false
    (:Completed
      (Utilities|FlowControl|Delay 2.0)
      (Audio|PlaySoundatLocation "/Game/Assets/audio/popsoundcue.popsoundcue" _returnvalue)
      (Effects|SpawnEmitteratLocation "/Game/Assets/spellbook/P_PuffSmoke.P_PuffSmoke" _returnvalue)
      (Rendering|SetVisibility (Variables|Default|Getspellbook_mesh) false false)
      (Utilities|FlowControl|Delay 5.0)
      (Components|DestroyComponent (Variables|Default|Getspellbook_mesh))
      (Class|BPIMyVRGamemode|Respawn(Message) (Variables|Default|GetGameMode)))))

(event EventBeginPlay
  (bind _outactors (Actor|GetAllActorsOfClass "/Game/Assets/player/myVRGamemode.myVRGamemode_C"))
  (Variables|Default|SetGameMode (Utilities|Array|Get(acopy) _outactors)))

(event EventPickUp
  (params (ActorToAttachTo :type Scene%20Component%20Object%20Reference))
  (Physics|SetSimulatePhysics (Variables|Default|Getspellbook_mesh) false)
  (Transformation|AttachComponentToComponent (VehicleSound|GetRootComponent) ActorToAttachTo "None" "KeepWorld" "KeepWorld" "KeepWorld" true))

(event Collision|EventHit
  (params (MyComp :type Primitive%20Component%20Object%20Reference) (Other :type Actor%20Object%20Reference) (OtherComp :type Primitive%20Component%20Object%20Reference) (bSelfMoved :type Boolean) (HitLocation :type Vector :default "0, 0, 0") (HitNormal :type Vector :default "0, 0, 0") (NormalImpulse :type Vector :default "0, 0, 0") (Hit :type Hit%20Result%20Structure%20%28by%20ref%29))
  (if (not (== Other (Game|Player|GetPlayerPawn 0)))
    (if (not (Variables|Default|GetisAudioExecuting))
      (Audio|PlaySoundatLocation "/Game/Assets/audio/bookslamCue.bookslamCue" (Transformation|GetWorldLocation (Variables|Default|Getspellbook_mesh)) "0.000000, 0, 0")
      (Variables|Default|SetisAudioExecuting true)
      (Utilities|FlowControl|Delay 2.0)
      (Variables|Default|SetisAudioExecuting false))))

(event EventDropOff
  (Physics|SetSimulatePhysics (Variables|Default|Getspellbook_mesh) true)
  (Transformation|DetachFromActor "KeepRelative" "KeepRelative" "KeepRelative"))

(fn ConstructionScript)