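; Goblin head prop Blueprint that turns to face the player and plays a goblin voice when its TurnHead event is called.
; After a two-second delay it plays the sound at the mesh and runs a timeline, restarting it if already finished.
; Each timeline update eases only the mesh's yaw toward the player, feeding the HeadTurn track into RInterpTo as delta time.
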(event EventBeginPlay)

(event Collision|EventActorBeginOverlap
  (params (OtherActor :type Actor%20Object%20Reference)))

(event EventTick
  (params (DeltaSeconds :type Float%20%28single-precision%29)))

(event EventTurnHead
  (bind _goblinheadturnanimation (Variables|Default|GetGoblinHeadTurnAnimation))
  (bind _staticmesh (Variables|Default|GetStaticMesh))
  (if (< (Components|Timeline|GetPlaybackPosition _goblinheadturnanimation) (Components|Timeline|GetTimelineLength _goblinheadturnanimation))
    (Utilities|FlowControl|Delay 2.0)
    (Audio|PlaySoundatLocation "/Game/Assets/audio/goblin_voice_Cue.goblin_voice_Cue" (Transformation|GetWorldLocation (Variables|Default|GetStaticMesh)))
    (bind _headturn (Timeline|GoblinHeadTurnAnimation Play)
      (:Update
        (Transformation|SetWorldRotation (Variables|Default|GetStaticMesh) (Math|Interpolation|RInterpTo (Transformation|GetWorldRotation _staticmesh) (Math|Rotator|MakeRotator 0.0 0.0 (.Yaw (Math|Rotator|BreakRotator (Math|Rotator|FindLookatRotation (Transformation|GetWorldLocation _staticmesh) (Transformation|GetActorLocation (Game|Player|GetPlayerPawn 0)))))) _headturn 0.05) false false)))
    (else
      (Utilities|FlowControl|Delay 2.0)
      (Audio|PlaySoundatLocation "/Game/Assets/audio/goblin_voice_Cue.goblin_voice_Cue" (Transformation|GetWorldLocation (Variables|Default|GetStaticMesh)))
      (Timeline|GoblinHeadTurnAnimation PlayFromStart))))

(fn ConstructionScript)